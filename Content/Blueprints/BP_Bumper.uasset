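; BP_Bumper is a pinball bumper that knocks an overlapping BP_Ball away from its center and awards score.
; On overlap it applies a velocity-change impulse, plays a hit sound and adds points through PinballGameMode in both Bump and the overlap handler.
; A timeline then drives the mechanism's vertical movement, light intensity and emissive boost on a dynamic material created in the Construction Script.
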(event `self.ReceiveActorBeginOverlap`
  (params (OtherActor :type "Actor Object Reference"))
  (bind _asbp_ball (cast `/Game/Blueprints/BP_Ball` OtherActor))
  (`self.Bump` _asbp_ball)
  (`GameplayStatics.SpawnSoundAttached` "/Game/Sounds/BumperHit.BumperHit" (`self.BumperBase`) "None" (0.0 0.0 0.0) (struct) "KeepRelativeOffset" false 1.0 1.0 0.0 null null)
  (bind _aspinball_game_mode (cast `/Game/Blueprints/PinballGameMode` (`GameplayStatics.GetGameMode`))
    (:`then`
      (`/Game/Blueprints/PinballGameMode.AddScore` _aspinball_game_mode 10.0)
      (bind (_direction _bump_alpha) (`Timeline|Timeline_0` :!via `PlayFromStart` :!label _label)
        (:`Update`
          (`SceneComponent.K2_SetRelativeLocation` (`self.BumperMechanism`) (`KismetMathLibrary.VLerp` (0.0 0.0 0.0) (0.0 0.0 -70.0) _bump_alpha) false false)
          (`LightComponent.SetIntensity` (`self.BumpLight`) (`KismetMathLibrary.Lerp` 0.0 5000.0 _bump_alpha))
          (`MaterialInstanceDynamic.SetScalarParameterValue` (`self.BumperTopMID`) "EmissiveBoost" (`KismetMathLibrary.Lerp` 0.0 20.0 _bump_alpha)))))
    (:`CastFailed`
      (goto _label :!via `PlayFromStart`))))

(event `Bump`
  (params (Ball :type "/Game/Blueprints/BP_Ball Object Reference"))
  (`PrimitiveComponent.AddImpulse` (`/Game/Blueprints/BP_Ball.Ball` Ball) (* (`KismetMathLibrary.GetDirectionUnitVector` (`self.K2_GetActorLocation`) (`self.K2_GetActorLocation` Ball)) (`self.BumperImpulse`)) "None" true)
  (bind _aspinball_game_mode (cast `/Game/Blueprints/PinballGameMode` (`GameplayStatics.GetGameMode`)))
  (`/Game/Blueprints/PinballGameMode.AddScore` _aspinball_game_mode 100.0))

(fn `UserConstructionScript`
  (bind _returnvalue (`PrimitiveComponent.CreateDynamicMaterialInstance` (`self.BumperBase`) 1 "/Game/Materials/M_BumperBase.M_BumperBase" "None"))
  (set `self.BumperTopMID` _returnvalue))