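; High score save object that holds a leaderboard array of score structs, trimmed to the top four entries.
; AddHighScore appends a new entry, calls SortSaveData, then resizes the array.
; SortSaveData does a descending selection sort, repeatedly moving the highest-scoring entry into a temporary array before copying it back.
; A lowest-score lookup mirrors the highest-score search but is not called within these graphs.
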(fn `AddHighScore`
  (params (NewScore :type "/Game/Blueprints/HIghScoreStruct Structure"))
  (bind _savestruct (`self.SaveStruct`))
  (`KismetArrayLibrary.Array_Add` (`self.SaveStruct`) NewScore)
  (`self.SortSaveData`)
  (`KismetArrayLibrary.Array_Resize` _savestruct (`KismetMathLibrary.Min` 4 (`KismetArrayLibrary.Array_Length` _savestruct))))

(fn `DetermineHighestScoreValue_0`
  (params (NewParam :type Boolean))
  (returns (HighestSoreStruct :type "/Game/Blueprints/HIghScoreStruct Structure") (HighestScoreIndex :type Integer))
  (locals (HighestScore :type "Float (double-precision)") (HighestIndex :type Integer))
  (bind _highestindex (`local.HighestIndex`))
  (for (_array_element _array_index) (`self.SaveStruct`)
    (if (== _array_index 0)
      (set `local.HighestScore` (`.Score_5_09DBE2ED4F55C1E2F8DE0C91C2AEAB1B` (break `/Game/Blueprints/HIghScoreStruct` _array_element)))
      (set `local.HighestIndex` _array_index)
      (elif (> (`.Score_5_09DBE2ED4F55C1E2F8DE0C91C2AEAB1B` (break `/Game/Blueprints/HIghScoreStruct` _array_element)) (`local.HighestScore`))
        (set `local.HighestScore` (`.Score_5_09DBE2ED4F55C1E2F8DE0C91C2AEAB1B` (break `/Game/Blueprints/HIghScoreStruct` _array_element)))
        (set `local.HighestIndex` _array_index))))
  (return (`|GetArrayItem` (`self.SaveStruct`) _highestindex) _highestindex))

(fn `DetermineLowestScoreValue`
  (params (NewParam :type Boolean))
  (returns (LowestSoreStruct :type "/Game/Blueprints/HIghScoreStruct Structure") (LowestScoreIndex :type Integer))
  (locals (LowestScore :type "Float (double-precision)") (LowestIndex :type Integer))
  (bind _lowestindex (`local.LowestIndex`))
  (for (_array_element _array_index) (`self.SaveStruct`)
    (if (== _array_index 0)
      (set `local.LowestScore` (`.Score_5_09DBE2ED4F55C1E2F8DE0C91C2AEAB1B` (break `/Game/Blueprints/HIghScoreStruct` _array_element)))
      (set `local.LowestIndex` _array_index)
      (elif (< (`.Score_5_09DBE2ED4F55C1E2F8DE0C91C2AEAB1B` (break `/Game/Blueprints/HIghScoreStruct` _array_element)) (`local.LowestScore`))
        (set `local.LowestScore` (`.Score_5_09DBE2ED4F55C1E2F8DE0C91C2AEAB1B` (break `/Game/Blueprints/HIghScoreStruct` _array_element)))
        (set `local.LowestIndex` _array_index))))
  (return (`|GetArrayItem` (`self.SaveStruct`) _lowestindex) _lowestindex))

(fn `SortSaveData`
  (locals (TemptSaveStruct :type "Array of /Game/Blueprints/HIghScoreStruct Structure"))
  (while (> (`KismetArrayLibrary.Array_Length` (`self.SaveStruct`)) 0)
    (bind (_highestsorestruct _highestscoreindex) (`self.DetermineHighestScoreValue_0` false))
    (`KismetArrayLibrary.Array_Add` (`local.TemptSaveStruct`) _highestsorestruct)
    (`KismetArrayLibrary.Array_Remove` (`self.SaveStruct`) _highestscoreindex))
  (set `self.SaveStruct` (`local.TemptSaveStruct`)))